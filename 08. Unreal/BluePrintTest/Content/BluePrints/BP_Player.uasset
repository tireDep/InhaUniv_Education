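; BP_Player is the player character Blueprint, handling third-person movement, camera look and zoom through legacy input action and axis events.
; Movement follows the control rotation's yaw only, while mouse axes drive controller pitch and yaw and a clamped spring arm length for zoom.
; Jump input starts and stops jumping, and holding the Walking action halves the max walk speed until released.
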(event `InputAction|Walking`
  (params (Key :type "Key Structure"))
  (bind _charactermovement (`self.CharacterMovement`))
  ;[1 1 1] Animation
  (:`Pressed`
    (set `CharacterMovementComponent.MaxWalkSpeed` 300.0 _charactermovement))
  (:`Released`
    (set `CharacterMovementComponent.MaxWalkSpeed` 600.0 _charactermovement)))

(event `InputAxis|MoveMouseY`
  (params (AxisValue :type "Float (single-precision)"))
  ;[1 1 1] Camera_Mouse
  (`self.AddControllerPitchInput` AxisValue))

(event `InputAction|Jumping`
  (params (Key :type "Key Structure"))
  ;[1 1 1] Camera_Mouse
  (:`Pressed`
    (`self.Jump`))
  (:`Released`
    (`self.StopJumping`)))

(event `InputAxis|MoveMouseX`
  (params (AxisValue :type "Float (single-precision)"))
  ;[1 1 1] Camera_Mouse
  (`self.AddControllerYawInput` AxisValue))

(event `InputAxis|ZoomMouse`
  (params (AxisValue :type "Float (single-precision)"))
  ;[1 1 1] Camera_Mouse
  (set `SpringArmComponent.TargetArmLength` (`KismetMathLibrary.FClamp` (+ (* AxisValue (`self.ZoomSpeed`)) (`SpringArmComponent.TargetArmLength` (`self.SpringArm`))) 200.0 600.0) (`self.SpringArm`)))

(event `InputAxis|MoveForward`
  (params (AxisValue :type "Float (single-precision)"))
  (bind (_returnvalue_roll _returnvalue_pitch _returnvalue_yaw) (`KismetMathLibrary.BreakRotator` (`self.GetControlRotation`)))
  ;[1 1 1] PlayerMove
  (`self.AddMovementInput` (`KismetMathLibrary.Vector_Normal2D` (`KismetMathLibrary.GetForwardVector` (`KismetMathLibrary.MakeRotator` 0.0 0.0 _returnvalue_yaw))) AxisValue))

(event `InputAxis|MoveRight`
  (params (AxisValue :type "Float (single-precision)"))
  (bind (_returnvalue_roll _returnvalue_pitch _returnvalue_yaw) (`KismetMathLibrary.BreakRotator` (`self.GetControlRotation`)))
  ;[1 1 1] PlayerMove
  (`self.AddMovementInput` (`KismetMathLibrary.Vector_Normal2D` (`KismetMathLibrary.GetRightVector` (`KismetMathLibrary.MakeRotator` 0.0 0.0 _returnvalue_yaw))) AxisValue))

(fn `NewFunction_0`)

(fn `UserConstructionScript`)